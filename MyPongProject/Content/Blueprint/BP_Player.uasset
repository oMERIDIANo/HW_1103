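; BP_Player is the player actor, moved side to side along the X axis by the Move input axis.
; Each axis event offsets it locally by Speed times the input, without sweep or delta-time scaling, and stores the truncated input in Direction.
; If the new world X reaches 300 or beyond either way, an opposite offset undoes that step to keep it within bounds.
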(event EventBeginPlay)

(event Input|AxisEvents|InputAxisMove
  (params (AxisValue :type Float%20%28single-precision%29))
  (bind _returnvalue (Input|AxisValues|GetMove))
  (Transformation|AddActorLocalOffset (Math|Vector|MakeVector (* (Variables|Default|GetSpeed) _returnvalue) 0.0 0.0) false false)
  (Variables|Default|SetDirection (Math|Float|Truncate _returnvalue))
  (if (>= (.X (Math|Vector|BreakVector (Transformation|GetActorLocation))) 3e+02)
    (Transformation|AddActorLocalOffset (* (Math|Vector|MakeVector (* (Variables|Default|GetSpeed) -1.0) 0.0 0.0) (Input|AxisValues|GetMove)) false false)
    (elif (<= (.X (Math|Vector|BreakVector (Transformation|GetActorLocation))) -3e+02)
      (Transformation|AddActorLocalOffset (* (Math|Vector|MakeVector (* (Variables|Default|GetSpeed) -1.0) 0.0 0.0) (Input|AxisValues|GetMove)) false false))))

(fn ConstructionScript)