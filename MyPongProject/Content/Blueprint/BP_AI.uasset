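; BP_AI is an AI-controlled actor that follows BP_InvisibleBall along the X axis.
; Each tick it looks up that actor, stores its position and calls SetDirection to choose +1 or -1; the zero case is unreachable.
; It moves by that local X offset with sweep, at a frame-rate-dependent speed.
; Exact-equality checks at the positive and negative X bounds nudge it one unit back inward.
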(event EventTick
  (params (DeltaSeconds :type Float%20%28single-precision%29))
  (bind _returnvalue (Actor|GetActorOfClass "/Game/Blueprint/BP_InvisibleBall.BP_InvisibleBall_C"))
  (Variables|Default|SetPosition (Transformation|GetActorLocation _returnvalue))
  (CallFunction|SetDirection)
  (Transformation|AddActorLocalOffset (Math|Vector|MakeVector (Math|Conversions|ToFloat(Integer) (Variables|Default|GetDirection)) 0.0 0.0) true false)
  (if (== (.X (Math|Vector|BreakVector (Transformation|GetActorLocation))) 3e+02)
    (Transformation|AddActorLocalOffset "-1.000000, 0, 0" false false)
    (elif (== (.X (Math|Vector|BreakVector (Transformation|GetActorLocation))) -3e+02)
      (Transformation|AddActorLocalOffset "1.000000, 0, 0" false false))))

(fn ConstructionScript)

(fn SetDirection
  (if (<= (.X (Math|Vector|BreakVector (Transformation|GetActorLocation))) (.X (Math|Vector|BreakVector (Variables|Default|GetPosition))))
    (Variables|Default|SetDirection 1)
    (elif (>= (.X (Math|Vector|BreakVector (Transformation|GetActorLocation))) (.X (Math|Vector|BreakVector (Variables|Default|GetPosition))))
      (Variables|Default|SetDirection -1)
      (else
        (Variables|Default|SetDirection 0)))))