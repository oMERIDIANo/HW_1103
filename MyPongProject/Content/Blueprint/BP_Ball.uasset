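; Pong-style ball that bounces between BP_Player and BP_AI, speeding up with each paddle hit.
; Paddle overlaps add randomized spin based on paddle direction, flip Y velocity and increment a hit count; barriers flip X.
; Player hits also launch BP_InvisibleBall from the ball's position at double velocity.
; Tick resets the ball when it passes either paddle's Y position, dividing velocity by the hit count and zeroing it.
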(event Collision|EventActorBeginOverlap
  (params (OtherActor :type Actor%20Object%20Reference))
  (bind _projectilemovement (Variables|Default|GetProjectileMovement))
  (bind _asbp_player (Utilities|Casting|CastToBP_Player OtherActor)
    (:then
      (CallFunction|HandleBounce (Variables|/Game/Blueprint/BP_Player.BP_Player_C|GetDirection _asbp_player))
      (bind _outactors (Actor|GetAllActorsOfClass "/Game/Blueprint/BP_InvisibleBall.BP_InvisibleBall_C"))
      (Transformation|SetActorLocation (Utilities|Array|Get(acopy) _outactors) (Transformation|GetActorLocation) false false)
      (Variables|/Script/Engine.MovementComponent|SetVelocity (Variables|/Game/Blueprint/BP_InvisibleBall.BP_InvisibleBall_C|GetProjectileMovement (Utilities|Array|Get(acopy) _outactors)) (* (Variables|/Script/Engine.MovementComponent|GetVelocity (Variables|Default|GetProjectileMovement)) "2.000000,2.000000, 0"))
      (Variables|/Script/Engine.MovementComponent|SetVelocity _projectilemovement (Math|Vector|MakeVector (* (.X (Math|Vector|BreakVector (Variables|/Script/Engine.MovementComponent|GetVelocity _projectilemovement))) (Variables|Default|GetSpeedUp)) (* (.Y (Math|Vector|BreakVector (Variables|/Script/Engine.MovementComponent|GetVelocity _projectilemovement))) (Variables|Default|GetSpeedUp)) 0.0) :!label _label)
      (bind _output_get (Variables|Default|SetCount (+ (Variables|Default|GetCount) 1)))
      (Development|PrintString (Utilities|String|ToString(Integer) _output_get)))
    (:CastFailed
      (bind _asbp_ai (Utilities|Casting|CastToBP_AI OtherActor)
        (:then
          (CallFunction|HandleBounce (Variables|/Game/Blueprint/BP_AI.BP_AI_C|GetDirection _asbp_ai))
          (goto _label))
        (:CastFailed
          (Utilities|Casting|CastToBP_Barrier OtherActor)
          (CallFunction|ReverseX))))))

(event EventTick
  (params (DeltaSeconds :type Float%20%28single-precision%29))
  (bind _projectilemovement (Variables|Default|GetProjectileMovement))
  (Variables|Default|SettimeSinceReversed (+ DeltaSeconds (Variables|Default|GettimeSinceReversed)))
  (bind _outofbounds (CallFunction|IsOutOfBounds))
  (if _outofbounds
    (Transformation|SetActorLocation "-50.000000,10.000000,50.000000" false false)
    (Variables|/Script/Engine.MovementComponent|SetVelocity _projectilemovement (Math|Vector|MakeVector (/ (.X (Math|Vector|BreakVector (Variables|/Script/Engine.MovementComponent|GetVelocity _projectilemovement))) (Math|Conversions|ToFloat(Integer) (Variables|Default|GetCount))) (/ (.Y (Math|Vector|BreakVector (Variables|/Script/Engine.MovementComponent|GetVelocity _projectilemovement))) (Math|Conversions|ToFloat(Integer) (Variables|Default|GetCount))) 0.0))
    (bind _output_get (Variables|Default|SetCount 0))
    (Development|PrintString (Utilities|String|ToString(Integer) _output_get))))

(fn ConstructionScript)

(fn AddSpin
  (params (Spin :type Float%20%28single-precision%29))
  (Variables|/Script/Engine.MovementComponent|SetVelocity (Variables|Default|GetProjectileMovement) (+ (Math|Vector|MakeVector Spin 0.0 0.0) (Variables|/Script/Engine.MovementComponent|GetVelocity (Variables|Default|GetProjectileMovement)))))

(fn ReverseY
  (if (>= (Variables|Default|GettimeSinceReversed) 0.0)
    (Variables|/Script/Engine.MovementComponent|SetVelocity (Variables|Default|GetProjectileMovement) (Math|Vector|MakeVector (.X (Math|Vector|BreakVector (Variables|/Script/Engine.MovementComponent|GetVelocity (Variables|Default|GetProjectileMovement)))) (* -1 (.Y (Math|Vector|BreakVector (Variables|/Script/Engine.MovementComponent|GetVelocity (Variables|Default|GetProjectileMovement))))) (.Z (Math|Vector|BreakVector (Variables|/Script/Engine.MovementComponent|GetVelocity (Variables|Default|GetProjectileMovement))))))
    (Development|PrintString "Reverse Y")
    (Variables|Default|SettimeSinceReversed 0.0)))

(fn ReverseX
  (if (>= (Variables|Default|GettimeSinceReversed) 0.0)
    (Variables|/Script/Engine.MovementComponent|SetVelocity (Variables|Default|GetProjectileMovement) (Math|Vector|MakeVector (* -1 (.X (Math|Vector|BreakVector (Variables|/Script/Engine.MovementComponent|GetVelocity (Variables|Default|GetProjectileMovement))))) (.Y (Math|Vector|BreakVector (Variables|/Script/Engine.MovementComponent|GetVelocity (Variables|Default|GetProjectileMovement)))) (.Z (Math|Vector|BreakVector (Variables|/Script/Engine.MovementComponent|GetVelocity (Variables|Default|GetProjectileMovement))))))
    (Development|PrintString "Reverse X")
    (Variables|Default|SettimeSinceReversed 0.0)))

(fn IsOutOfBounds
  (bind _outactors (Actor|GetAllActorsOfClass "/Game/Blueprint/BP_Player.BP_Player_C"))
  (if (<= (.Y (Math|Vector|BreakVector (Transformation|GetActorLocation))) (.Y (Math|Vector|BreakVector (Transformation|GetActorLocation (Utilities|Array|Get(acopy) _outactors)))))
    _
    (else
      (bind _outactors_2 (Actor|GetAllActorsOfClass "/Game/Blueprint/BP_AI.BP_AI_C"))
      (if (>= (.Y (Math|Vector|BreakVector (Transformation|GetActorLocation))) (.Y (Math|Vector|BreakVector (Transformation|GetActorLocation (Utilities|Array|Get(acopy) _outactors_2)))))
        _
        (else
          (return false)))))
  (return true))

(fn HandleBounce
  (params (Selection :type Integer))
  (bind _returnvalue (Math|Random|RandomFloatinRange -5e+01 5e+01))
  (switch int Selection
    (:-1
      (CallFunction|AddSpin (+ _returnvalue -125.0)))
    (:0
      (CallFunction|AddSpin (Math|Random|RandomFloatinRange -15.0 15.0)))
    (:1
      (CallFunction|AddSpin (+ _returnvalue 1.0))))
  (CallFunction|ReverseY))